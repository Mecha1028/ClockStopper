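; Test player character for twin-stick play, with movement relative to camera yaw and the body turning toward the cursor's hit point.
; Holding left mouse switches to orbiting the spring arm within clamped angles, pausing aim.
; Number keys flag camera tuning: the mouse wheel adjusts FOV, while position and rotation step events have no callers here.
; Damage and timer events deplete health and time, calling empty death and shutdown stubs.
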(event Custom|ChangeModel
  (Components|StaticMesh|SetStaticMesh (Variables|Default|GetPlayerBody) (Variables|Default|GetNewPlayerMesh))
  (Components|StaticMesh|SetStaticMesh (Variables|Default|GetPlayerWeapon) (Variables|Default|GetNewWeaponMesh)))

(event Custom|POSAdd
  ;[0.15 0.15 0.15 0.5] change position and rotation in positive direction
  (if (Variables|Camera|GetChangePOSX)
    (bind _result (Math|Float|IncrementFloat (Variables|Camera|GetPOSX))
      (:%20%20
        (Variables|Camera|SetPOSX (Math|Float|Clamp(Float) _result -1e+02 1e+02))
        (CallFunction|ChangeCam :!label _label)))
    (elif (Variables|Camera|GetChangePOSY)
      (bind _result_2 (Math|Float|IncrementFloat (Variables|Camera|GetPOSY))
        (:%20%20
          (Variables|Camera|SetPOSY (Math|Float|Clamp(Float) _result_2 -1e+02 1e+02))
          (goto _label)))
      (elif (Variables|Camera|GetChangePOSZ)
        (bind _result_3 (Math|Float|IncrementFloat (Variables|Camera|GetPOSZ))
          (:%20%20
            (Variables|Camera|SetPOSZ (Math|Float|Clamp(Float) _result_3 -1e+02 1e+02))
            (goto _label)))))))

(event Custom|PlayerShutdown
  ;[0.15 0.15 0.15 0.5] Health and Time logic
)

(event Custom|TimerChange
  ;[0.15 0.15 0.15 0.5] Health and Time logic
  (bind _output_get (Variables|Status|SetPlayerTime (+ (Variables|Status|GetPlayerTime) (Variables|Status|GetExternalTimeModifier))))
  (if (<= _output_get 0.0)
    (CallFunction|PlayerShutdown)))

(event Custom|RotateYMouse
  ;[0.15 0.15 0.15 0.5] sets and clamps camera angle
  (if (Variables|Default|GetCanChangeAngle)
    (Variables|Default|SetCanTwinStick false)
    (Variables|Camera|SetROTY (Math|Float|Clamp(Float) (+ (* (Variables|Default|GetMouseYREF) (Variables|Default|GetMouseSensitivity)) (Variables|Camera|GetROTY)) -8e+01 -1e+01))
    (CallFunction|ChangeCam)
    (else
      (Variables|Default|SetCanTwinStick true))))

(event Custom|RotateXMouse
  ;[0.15 0.15 0.15 0.5] sets and clamps camera angle
  (if (Variables|Default|GetCanChangeAngle)
    (Variables|Default|SetCanTwinStick false)
    (Variables|Camera|SetROTZ (Math|Float|Clamp(Float) (+ (* (Variables|Default|GetMouseXREF) (Variables|Default|GetMouseSensitivity)) (Variables|Camera|GetROTZ)) -9e+01 9e+01))
    (CallFunction|ChangeCam)
    (else
      (Variables|Default|SetCanTwinStick true))))

(event Custom|TwinStickEvent
  (bind _returnvalue (Transformation|GetActorLocation))
  (bind _bp_td_controller (Variables|Default|GetBP%20TD%20Controller))
  (bind (_hitresult _returnvalue_2) (Game|Player|GetHitResultUnderCursorbyChannel _bp_td_controller "TraceTypeQuery1" true))
  (if (and _returnvalue_2 (Variables|Default|GetCanTwinStick))
    (bind _output_get (Variables|Default|SetHit%20Result%20Location (.location _hitresult)))
    (Transformation|SetWorldRotation (Variables|Default|GetPlayerBody) (Math|Interpolation|RInterpTo (Transformation|GetActorRotation) (Math|Rotator|FindLookatRotation (Math|Vector|MakeVector (.x _returnvalue) (.y _returnvalue) (.Z (Math|Vector|BreakVector _output_get))) (Math|Vector|MakeVector (.X (Math|Vector|BreakVector _output_get)) (.Y (Math|Vector|BreakVector _output_get)) (.Z (Math|Vector|BreakVector _output_get)))) (Utilities|Time|GetWorldDeltaSeconds) 0.0) false false)))

(event Custom|ROTAdd
  ;[0.15 0.15 0.15 0.5] change position and rotation in positive direction
  (if (Variables|Camera|GetChangeRotX)
    (bind _result (Math|Float|IncrementFloat (Variables|Camera|GetROTX))
      (:%20%20
        (Variables|Camera|SetROTX (Math|Float|Clamp(Float) _result -1e+02 1e+02))
        (CallFunction|ChangeCam :!label _label)))
    (elif (Variables|Camera|GetChangeRotY)
      (bind _result_2 (Math|Float|IncrementFloat (Variables|Camera|GetROTY))
        (:%20%20
          (Variables|Camera|SetROTY (Math|Float|Clamp(Float) _result_2 -1e+02 1e+02))
          (goto _label)))
      (elif (Variables|Camera|GetChangeRotZ)
        (bind _result_3 (Math|Float|IncrementFloat (Variables|Camera|GetROTZ))
          (:%20%20
            (Variables|Camera|SetROTZ (Math|Float|Clamp(Float) _result_3 -1e+02 1e+02))
            (goto _label)))))))

(event Custom|POSMin
  ;[0.15 0.15 0.15 0.5] change position and rotation in negative direction
  (if (Variables|Camera|GetChangePOSX)
    (bind _result (Math|Float|DecrementFloat (Variables|Camera|GetPOSX))
      (:%20%20
        (Variables|Camera|SetPOSX (Math|Float|Clamp(Float) _result -1e+02 1e+02))
        (CallFunction|ChangeCam :!label _label)))
    (elif (Variables|Camera|GetChangePOSY)
      (bind _result_2 (Math|Float|DecrementFloat (Variables|Camera|GetPOSY))
        (:%20%20
          (Variables|Camera|SetPOSY (Math|Float|Clamp(Float) _result_2 -1e+02 1e+02))
          (goto _label)))
      (elif (Variables|Camera|GetChangePOSZ)
        (bind _result_3 (Math|Float|DecrementFloat (Variables|Camera|GetPOSZ))
          (:%20%20
            (Variables|Camera|SetPOSZ (Math|Float|Clamp(Float) _result_3 -1e+02 1e+02))
            (goto _label)))))))

(event Custom|ROTMin
  ;[0.15 0.15 0.15 0.5] change position and rotation in negative direction
  (if (Variables|Camera|GetChangeRotX)
    (bind _result (Math|Float|DecrementFloat (Variables|Camera|GetROTX))
      (:%20%20
        (Variables|Camera|SetROTX (Math|Float|Clamp(Float) _result -1e+02 1e+02))
        (CallFunction|ChangeCam :!label _label)))
    (elif (Variables|Camera|GetChangeRotY)
      (bind _result_2 (Math|Float|DecrementFloat (Variables|Camera|GetROTY))
        (:%20%20
          (Variables|Camera|SetROTY (Math|Float|Clamp(Float) _result_2 -1e+02 1e+02))
          (goto _label)))
      (elif (Variables|Camera|GetChangeRotZ)
        (bind _result_3 (Math|Float|DecrementFloat (Variables|Camera|GetROTZ))
          (:%20%20
            (Variables|Camera|SetROTZ (Math|Float|Clamp(Float) _result_3 -1e+02 1e+02))
            (goto _label)))))))

(event Custom|AddFOV
  (bind _camera (Variables|Default|GetCamera))
  (bind _fieldofview (Variables|/Script/Engine.CameraComponent|GetFieldOfView _camera))
  (if (Variables|Camera|GetChangeFOV)
    (Math|Float|DecrementFloat _fieldofview
      (:%20%20
        (Camera|SetFieldOfView _camera (Math|Float|Clamp(Float) _fieldofview 0.0 1e+03))))))

(event Custom|MinFOV
  (bind _camera (Variables|Default|GetCamera))
  (bind _fieldofview (Variables|/Script/Engine.CameraComponent|GetFieldOfView _camera))
  (if (Variables|Camera|GetChangeFOV)
    (Math|Float|IncrementFloat _fieldofview
      (:%20%20
        (Camera|SetFieldOfView _camera (Math|Float|Clamp(Float) _fieldofview 0.0 1e+03))))))

(event Custom|TakeDamage
  ;[0.15 0.15 0.15 0.5] Health and Time logic
  (bind _output_get (Variables|Status|SetPlayerHealth (- (Variables|Status|GetPlayerHealth) (Variables|Status|GetExternalDamageNum))))
  (if (<= _output_get 0.0)
    (CallFunction|PlayerDeath)))

(event Custom|ChangeCam
  ;[0.15 0.15 0.15 0.5] alter position of camera and rotation of springarm
  (Transformation|SetRelativeRotation (Variables|Default|GetSpringArm) (Math|Rotator|MakeRotator (Variables|Camera|GetROTX) (Variables|Camera|GetROTY) (Variables|Camera|GetROTZ)) false false)
  (Transformation|SetRelativeLocation (Variables|Default|GetCamera) (Math|Vector|MakeVector (Variables|Camera|GetPOSX) (Variables|Camera|GetPOSY) (Variables|Camera|GetPOSZ)) false true))

(event Custom|PlayerDeath
  ;[0.15 0.15 0.15 0.5] Health and Time logic
)

(event EventBeginPlay
  (bind _asbp_td_controller (Utilities|Casting|CastToBP_TD_Controller (Game|GetPlayerController 0)))
  (bind _output_get (Variables|Default|SetBP%20TD%20Controller _asbp_td_controller))
  (Pawn|SetControlRotation _output_get (Math|Rotator|MakeRotator 0.0 3e+02 0.0))
  (Variables|/Script/Engine.PlayerController|SetbShowMouseCursor _output_get false)
  (Input|AddMappingContext (PlayerController|LocalPlayerSubsystems|GetEnhancedInputLocalPlayerSubsystem _output_get) 0 0 "(bIgnoreAllPressedKeysUntilRelease=True,bForceImmediately=False,bNotifyUserSettings=False)"))

(event EventTick
  (params (DeltaSeconds :type Float%20%28single-precision%29))
  (CallFunction|TwinStickEvent))

(event Input|AxisEvents|InputAxisForward/Backward
  (params (AxisValue :type Float%20%28single-precision%29))
  (Pawn|Input|AddMovementInput (Math|Vector|GetForwardVector (Math|Rotator|MakeRotator 0.0 0.0 (+ (Variables|Camera|GetROTZ) (.yaw (Pawn|GetControlRotation :!class /Script/Engine.Pawn))))) AxisValue false))

(event Input|AxisEvents|InputAxisLeft/Right
  (params (AxisValue :type Float%20%28single-precision%29))
  (bind _returnvalue (Pawn|GetControlRotation :!class /Script/Engine.Pawn))
  (Pawn|Input|AddMovementInput (Math|Vector|GetRightVector (Math|Rotator|MakeRotator (.roll _returnvalue) 0.0 (+ (Variables|Camera|GetROTZ) (.yaw _returnvalue)))) AxisValue false))

(event Input|AxisEvents|InputAxisCamup/Down
  (params (AxisValue :type Float%20%28single-precision%29))
  ;[0.15 0.15 0.15 0.5] accepts input from cam axis
  (Variables|Default|SetMouseYREF AxisValue)
  (CallFunction|RotateYMouse))

(event Input|AxisEvents|InputAxisCamLeft/Right
  (params (AxisValue :type Float%20%28single-precision%29))
  ;[0.15 0.15 0.15 0.5] accepts input from cam axis
  (Variables|Default|SetMouseXREF AxisValue)
  (CallFunction|RotateXMouse))

(event Input|KeyboardEvents|7
  (params (Key :type Key%20Structure :default "None"))
  ;[0.15 0.15 0.15 0.5] select direction to be changed
  (:Pressed
    (Variables|Camera|SetChangeFOV true))
  (:Released
    (Variables|Camera|SetChangeFOV false)))

(event Input|MouseEvents|LeftMouseButton
  (params (Key :type Key%20Structure :default "None"))
  ;[0.15 0.15 0.15 0.5] flag for if the player wants to change cam angle
  (:Pressed
    (Variables|Default|SetCanChangeAngle true))
  (:Released
    (Variables|Default|SetCanChangeAngle false)))

(event Input|KeyboardEvents|1
  (params (Key :type Key%20Structure :default "None"))
  ;[0.15 0.15 0.15 0.5] select direction to be changed
  (:Pressed
    (Variables|Camera|SetChangeRotX true))
  (:Released
    (Variables|Camera|SetChangeRotX false)))

(event Input|KeyboardEvents|2
  (params (Key :type Key%20Structure :default "None"))
  ;[0.15 0.15 0.15 0.5] select direction to be changed
  (:Pressed
    (Variables|Camera|SetChangeRotY true))
  (:Released
    (Variables|Camera|SetChangeRotY false)))

(event Input|KeyboardEvents|3
  (params (Key :type Key%20Structure :default "None"))
  ;[0.15 0.15 0.15 0.5] select direction to be changed
  (:Pressed
    (Variables|Camera|SetChangeRotZ true))
  (:Released
    (Variables|Camera|SetChangeRotZ false)))

(event Input|KeyboardEvents|4
  (params (Key :type Key%20Structure :default "None"))
  ;[0.15 0.15 0.15 0.5] select direction to be changed
  (:Pressed
    (Variables|Camera|SetChangePOSX true))
  (:Released
    (Variables|Camera|SetChangePOSX false)))

(event Input|KeyboardEvents|5
  (params (Key :type Key%20Structure :default "None"))
  ;[0.15 0.15 0.15 0.5] select direction to be changed
  (:Pressed
    (Variables|Camera|SetChangePOSY true))
  (:Released
    (Variables|Camera|SetChangePOSY false)))

(event Input|KeyboardEvents|6
  (params (Key :type Key%20Structure :default "None"))
  ;[0.15 0.15 0.15 0.5] select direction to be changed
  (:Pressed
    (Variables|Camera|SetChangePOSZ true))
  (:Released
    (Variables|Camera|SetChangePOSZ false)))

(event Input|MouseEvents|MouseWheelDown
  (params (Key :type Key%20Structure :default "None"))
  (:Pressed
    (CallFunction|MinFOV)))

(event Input|MouseEvents|MouseWheelUp
  (params (Key :type Key%20Structure :default "None"))
  (:Pressed
    (CallFunction|AddFOV)))

(fn ConstructionScript)