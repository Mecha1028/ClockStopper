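; Game manager that procedurally builds a level from rooms at startup and applies stored player and weapon meshes to the character.
; BeginPlay spawns the start room, then the first Tick loops synchronously, attaching random RoomList rooms at random open exits.
; Overlap boxes reject colliding rooms, destroying them and removing their exits.
; Successful placements refund the NumOfGen counter, so it effectively limits failed attempts rather than room count.
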(event Custom|SpawnStartRoom
  (bind _returnvalue (Game|SpawnActorfromClass "/Game/Jack/Blueprint/rooms/BP_MasterRoom.BP_MasterRoom_C" (Transformation|GetWorldTransform (Variables|Default|GetDefaultSceneRoot)) "AlwaysSpawn" "MultiplyWithRoot" 0 0))
  (Utilities|Array|AppendArray (Variables|Default|GetExitList) (Components|GetChildrenComponents (Variables|/Game/Jack/Blueprint/rooms/BP_MasterRoom.BP_MasterRoom_C|GetExitsFolder _returnvalue) false)))

(event Custom|SpawnNextRoom
  (bind _exitlist (Variables|Default|GetExitList))
  (if (Variables|Default|GetGenBool)
    (bind _output_get (Variables|Default|SetSelectedExit (.OutItem (Utilities|Array|Random (Variables|Default|GetExitList)))))
    (bind _returnvalue (Game|SpawnActorfromClass (.OutItem (Utilities|Array|Random (Variables|Default|GetRoomList))) (Math|Transform|MakeTransform (Transformation|GetWorldLocation _output_get) (Transformation|GetWorldRotation _output_get) "1.000000,1.000000,1.000000") "AlwaysSpawn" "MultiplyWithRoot" 0 0))
    (bind _asbp_master_room (Utilities|Casting|CastToBP_MasterRoom _returnvalue))
    (bind _output_get_2 (Variables|Default|SetMasterRoomREF _asbp_master_room))
    (Variables|Default|SetExitsREF (Components|GetChildrenComponents (Variables|/Game/Jack/Blueprint/rooms/BP_MasterRoom.BP_MasterRoom_C|GetExitsFolder _output_get_2) false))
    (Utilities|Array|AppendArray _exitlist (Components|GetChildrenComponents (Variables|/Game/Jack/Blueprint/rooms/BP_MasterRoom.BP_MasterRoom_C|GetExitsFolder _output_get_2) false))
    (CallFunction|CheckOverlap)
    (Utilities|Array|RemoveItem _exitlist (Variables|Default|GetSelectedExit))))

(event Custom|GetCharREF
  (bind _returnvalue (Actor|GetActorOfClass "/Game/Jack/Blueprint/GameMode/BP_Test_Character.BP_Test_Character_C"))
  (Utilities|IsValid _returnvalue
    (:Is%20Valid
      (bind _output_get (Variables|Default|SetCharacterREF _returnvalue))
      (Variables|/Game/Jack/Blueprint/GameMode/BP_Test_Character.BP_Test_Character_C|SetNewPlayerMesh _output_get (Variables|Default|GetGMNewPlayerMesh))
      (Variables|/Game/Jack/Blueprint/GameMode/BP_Test_Character.BP_Test_Character_C|SetNewWeaponMesh (Variables|Default|GetCharacterREF) (Variables|Default|GetGMNewWeaponMesh))
      (Default|ChangeModel (Variables|Default|GetCharacterREF)))))

(event Custom|AddOverlapRooms
  ;[0.15 0.15 0.15 0.5] check for overlapping rooms
  (for _array_element (Components|GetChildrenComponents (Variables|/Game/Jack/Blueprint/rooms/BP_MasterRoom.BP_MasterRoom_C|GetOverlapFolder (Variables|Default|GetMasterRoomREF)) false)
    (bind _asbox_collision (Utilities|Casting|CastToBoxComponent _array_element))
    (Utilities|Array|AppendArray (Variables|Default|GetOverlapList) (Class|PrimitiveComponent|GetOverlappingComponents _asbox_collision))))

(event Custom|checkOverlap
  (bind _masterroomref (Variables|Default|GetMasterRoomREF))
  (bind _overlaplist (Variables|Default|GetOverlapList))
  (CallFunction|AddOverlapRooms)
  (if (Utilities|Array|IsNotEmpty (Variables|Default|GetOverlapList))
    (Utilities|Array|Clear _overlaplist)
    (for _array_element (Variables|Default|GetExitsREF)
      (Utilities|Array|RemoveItem (Variables|Default|GetExitList) _array_element)
      (Utilities|IsValid _masterroomref
        (:Is%20Valid
          (Actor|DestroyActor _masterroomref))))
    (else
      (Utilities|Array|Clear _overlaplist)
      (Variables|Default|SetNumOfGen (+ (Variables|Default|GetNumOfGen) 1.0)))))

(event EventTick
  (params (DeltaSeconds :type Float%20%28single-precision%29))
  (if (Variables|Default|GetFirstRoomSpawned)
    (while (Variables|Default|GetGenBool)
      (bind _output_get (Variables|Default|SetNumOfGen (- (Variables|Default|GetNumOfGen) 1.0)))
      (Variables|Default|SetGenBool (> _output_get 0.0))
      (CallFunction|SpawnNextRoom))
    (Development|PrintString "Done")
    (Variables|Default|SetFirstRoomSpawned false)))

(event EventBeginPlay
  (CallFunction|SpawnStartRoom)
  (Variables|Default|SetFirstRoomSpawned true)
  (CallFunction|GetCharREF))

(fn ConstructionScript)