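; Test character for tuning a spring-arm camera live, with basic movement relative to control rotation and a ChangeModel event that swaps the body mesh.
; Held number keys 1-7 select a rotation axis, position axis or FOV, and the mouse wheel steps the selected value.
; Tick applies the clamped rotation to the spring arm and clamped position to the camera.
; FOV applies immediately, unclamped, with wheel-up narrowing it.
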(event Custom|ChangeModel
  (Components|StaticMesh|SetStaticMesh (Variables|Default|GetTestBody) (Variables|Default|GetNew%20Mesh)))

(event Custom|POSAdd
  ;[0.15 0.15 0.15 0.5] change position and rotation in positive direction
  (if (Variables|Camera|GetChangePOSX)
    (bind _result (Math|Float|IncrementFloat (Variables|Camera|GetPOSX))
      (:%20%20
        (Variables|Camera|SetPOSX (Math|Float|Clamp(Float) _result -1e+02 1e+02))))
    (elif (Variables|Camera|GetChangePOSY)
      (bind _result_2 (Math|Float|IncrementFloat (Variables|Camera|GetPOSY))
        (:%20%20
          (Variables|Camera|SetPOSY (Math|Float|Clamp(Float) _result_2 -1e+02 1e+02))))
      (elif (Variables|Camera|GetChangePOSZ)
        (bind _result_3 (Math|Float|IncrementFloat (Variables|Camera|GetPOSZ))
          (:%20%20
            (Variables|Camera|SetPOSZ (Math|Float|Clamp(Float) _result_3 -1e+02 1e+02))))))))

(event Custom|ROTAdd
  ;[0.15 0.15 0.15 0.5] change position and rotation in positive direction
  (if (Variables|Camera|GetChangeRotX)
    (bind _result (Math|Float|IncrementFloat (Variables|Camera|GetROTX))
      (:%20%20
        (Variables|Camera|SetROTX (Math|Float|Clamp(Float) _result -1e+02 1e+02))))
    (elif (Variables|Camera|GetChangeRotY)
      (bind _result_2 (Math|Float|IncrementFloat (Variables|Camera|GetROTY))
        (:%20%20
          (Variables|Camera|SetROTY (Math|Float|Clamp(Float) _result_2 -1e+02 1e+02))))
      (elif (Variables|Camera|GetChangeRotZ)
        (bind _result_3 (Math|Float|IncrementFloat (Variables|Camera|GetROTZ))
          (:%20%20
            (Variables|Camera|SetROTZ (Math|Float|Clamp(Float) _result_3 -1e+02 1e+02))))))))

(event Custom|POSMin
  ;[0.15 0.15 0.15 0.5] change position and rotation in negative direction
  (if (Variables|Camera|GetChangePOSX)
    (bind _result (Math|Float|DecrementFloat (Variables|Camera|GetPOSX))
      (:%20%20
        (Variables|Camera|SetPOSX (Math|Float|Clamp(Float) _result -1e+02 1e+02))))
    (elif (Variables|Camera|GetChangePOSY)
      (bind _result_2 (Math|Float|DecrementFloat (Variables|Camera|GetPOSY))
        (:%20%20
          (Variables|Camera|SetPOSY (Math|Float|Clamp(Float) _result_2 -1e+02 1e+02))))
      (elif (Variables|Camera|GetChangePOSZ)
        (bind _result_3 (Math|Float|DecrementFloat (Variables|Camera|GetPOSZ))
          (:%20%20
            (Variables|Camera|SetPOSZ (Math|Float|Clamp(Float) _result_3 -1e+02 1e+02))))))))

(event Custom|ROTMin
  ;[0.15 0.15 0.15 0.5] change position and rotation in negative direction
  (if (Variables|Camera|GetChangeRotX)
    (bind _result (Math|Float|DecrementFloat (Variables|Camera|GetROTX))
      (:%20%20
        (Variables|Camera|SetROTX (Math|Float|Clamp(Float) _result -1e+02 1e+02))))
    (elif (Variables|Camera|GetChangeRotY)
      (bind _result_2 (Math|Float|DecrementFloat (Variables|Camera|GetROTY))
        (:%20%20
          (Variables|Camera|SetROTY (Math|Float|Clamp(Float) _result_2 -1e+02 1e+02))))
      (elif (Variables|Camera|GetChangeRotZ)
        (bind _result_3 (Math|Float|DecrementFloat (Variables|Camera|GetROTZ))
          (:%20%20
            (Variables|Camera|SetROTZ (Math|Float|Clamp(Float) _result_3 -1e+02 1e+02))))))))

(event Custom|AddFOV
  (if (Variables|Default|GetChangeFOV)
    (Math|Float|DecrementFloat (Variables|Default|GetCamFOV)
      (:%20%20
        (Camera|SetFieldOfView (Variables|Default|GetCamera) (Variables|Default|GetCamFOV))))))

(event Custom|MinFOV
  (if (Variables|Default|GetChangeFOV)
    (Math|Float|IncrementFloat (Variables|Default|GetCamFOV)
      (:%20%20
        (Camera|SetFieldOfView (Variables|Default|GetCamera) (Variables|Default|GetCamFOV))))))

(event EventTick
  (params (DeltaSeconds :type Float%20%28single-precision%29))
  ;[0.15 0.15 0.15 0.5] alter position of camera and rotation of springarm
  (Transformation|SetRelativeRotation (Variables|Default|GetSpringArm) (Math|Rotator|MakeRotator (Variables|Camera|GetROTX) (Variables|Camera|GetROTY) (Variables|Camera|GetROTZ)) false false)
  (Transformation|SetRelativeLocation (Variables|Default|GetCamera) (Math|Vector|MakeVector (Variables|Camera|GetPOSX) (Variables|Camera|GetPOSY) (Variables|Camera|GetPOSZ)) false true))

(event Input|AxisEvents|InputAxisForward/Backward
  (params (AxisValue :type Float%20%28single-precision%29))
  (Pawn|Input|AddMovementInput (Math|Vector|GetForwardVector (Math|Rotator|MakeRotator 0.0 0.0 (.yaw (Pawn|GetControlRotation :!class /Script/Engine.Pawn)))) AxisValue false))

(event Input|AxisEvents|InputAxisLeft/Right
  (params (AxisValue :type Float%20%28single-precision%29))
  (bind _returnvalue (Pawn|GetControlRotation :!class /Script/Engine.Pawn))
  (Pawn|Input|AddMovementInput (Math|Vector|GetRightVector (Math|Rotator|MakeRotator (.roll _returnvalue) 0.0 (.yaw _returnvalue))) AxisValue false))

(event Input|KeyboardEvents|7
  (params (Key :type Key%20Structure :default "None"))
  ;[0.15 0.15 0.15 0.5] select direction to be changed
  (:Pressed
    (Variables|Default|SetChangeFOV true))
  (:Released
    (Variables|Default|SetChangeFOV false)))

(event Input|KeyboardEvents|1
  (params (Key :type Key%20Structure :default "None"))
  ;[0.15 0.15 0.15 0.5] select direction to be changed
  (:Pressed
    (Variables|Camera|SetChangeRotX true))
  (:Released
    (Variables|Camera|SetChangeRotX false)))

(event Input|KeyboardEvents|2
  (params (Key :type Key%20Structure :default "None"))
  ;[0.15 0.15 0.15 0.5] select direction to be changed
  (:Pressed
    (Variables|Camera|SetChangeRotY true))
  (:Released
    (Variables|Camera|SetChangeRotY false)))

(event Input|KeyboardEvents|3
  (params (Key :type Key%20Structure :default "None"))
  ;[0.15 0.15 0.15 0.5] select direction to be changed
  (:Pressed
    (Variables|Camera|SetChangeRotZ true))
  (:Released
    (Variables|Camera|SetChangeRotZ false)))

(event Input|KeyboardEvents|4
  (params (Key :type Key%20Structure :default "None"))
  ;[0.15 0.15 0.15 0.5] select direction to be changed
  (:Pressed
    (Variables|Camera|SetChangePOSX true))
  (:Released
    (Variables|Camera|SetChangePOSX false)))

(event Input|KeyboardEvents|5
  (params (Key :type Key%20Structure :default "None"))
  ;[0.15 0.15 0.15 0.5] select direction to be changed
  (:Pressed
    (Variables|Camera|SetChangePOSY true))
  (:Released
    (Variables|Camera|SetChangePOSY false)))

(event Input|KeyboardEvents|6
  (params (Key :type Key%20Structure :default "None"))
  ;[0.15 0.15 0.15 0.5] select direction to be changed
  (:Pressed
    (Variables|Camera|SetChangePOSZ true))
  (:Released
    (Variables|Camera|SetChangePOSZ false)))

(event Input|MouseEvents|MouseWheelDown
  (params (Key :type Key%20Structure :default "None"))
  (:Pressed
    (CallFunction|ROTMin)
    (CallFunction|POSMin)
    (CallFunction|MinFOV)))

(event Input|MouseEvents|MouseWheelUp
  (params (Key :type Key%20Structure :default "None"))
  (:Pressed
    (CallFunction|ROTAdd)
    (CallFunction|POSAdd)
    (CallFunction|AddFOV)))

(fn ConstructionScript)