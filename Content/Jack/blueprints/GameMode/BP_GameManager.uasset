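; Game manager that applies a new mesh to the test character and procedurally builds a level from room Blueprints at startup.
; BeginPlay spawns BP_Room1 at the manager's transform and collects its exit components into ExitList.
; The first Tick then loops on a countdown, attaching random RoomList rooms at random open exits, adding their exits and removing the used one.
; Rooms always spawn, with no overlap checks.
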(event Custom|SpawnStartRoom
  (bind _returnvalue (Game|SpawnActorfromClass "/Game/Jack/blueprints/BP_Room1.BP_Room1_C" (Transformation|GetWorldTransform (Variables|Default|GetDefaultSceneRoot)) "AlwaysSpawn" "MultiplyWithRoot" 0 0))
  (Utilities|Array|AppendArray (Variables|Default|GetExitList) (Components|GetChildrenComponents (Variables|/Game/Jack/blueprints/BP_Room1.BP_Room1_C|GetExitsFolder_0 _returnvalue) false)))

(event Custom|SpawnNextRoom
  (bind _exitlist (Variables|Default|GetExitList))
  (bind _output_get (Variables|Default|SetSelectedExit (.OutItem (Utilities|Array|Random (Variables|Default|GetExitList)))))
  (bind _returnvalue (Game|SpawnActorfromClass (.OutItem (Utilities|Array|Random (Variables|Default|GetRoomList))) (Math|Transform|MakeTransform (Transformation|GetWorldLocation _output_get) (Transformation|GetWorldRotation _output_get) "1.000000,1.000000,1.000000") "AlwaysSpawn" "MultiplyWithRoot" 0 0))
  (bind _asbp_master_room (Utilities|Casting|CastToBP_MasterRoom _returnvalue))
  (bind _output_get_2 (Variables|Default|SetLatestRoom _asbp_master_room))
  (Utilities|Array|AppendArray _exitlist (Components|GetChildrenComponents (Variables|/Game/Jack/blueprints/BP_MasterRoom.BP_MasterRoom_C|GetExitsFolder _output_get_2) false))
  (Utilities|Array|RemoveItem _exitlist (Variables|Default|GetSelectedExit)))

(event EventTick
  (params (DeltaSeconds :type Float%20%28single-precision%29))
  (if (Variables|Default|GetFirstRoomSpawned)
    (while (Variables|Default|GetGenBool)
      (bind _output_get (Variables|Default|SetNumOfGen (- (Variables|Default|GetNumOfGen) 1.0)))
      (Variables|Default|SetGenBool (> _output_get 0.0))
      (CallFunction|SpawnNextRoom))
    (Development|PrintString "Done")
    (Variables|Default|SetFirstRoomSpawned false)))

(event EventBeginPlay
  (bind _returnvalue (Actor|GetActorOfClass "/Game/Jack/blueprints/GameMode/BP_Test_Character.BP_Test_Character_C"))
  (bind _output_get (Variables|Default|SetcharREF _returnvalue))
  (Variables|/Game/Jack/blueprints/GameMode/BP_Test_Character.BP_Test_Character_C|SetNew%20Mesh _output_get (Variables|Default|GetGMNewMesh))
  (Default|ChangeModel (Variables|Default|GetcharREF))
  (CallFunction|SpawnStartRoom)
  (Variables|Default|SetFirstRoomSpawned true))

(fn ConstructionScript)